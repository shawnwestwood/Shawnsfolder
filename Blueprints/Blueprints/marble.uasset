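; Marble Blueprint for a physics sphere that the player rolls with the mouse and can reset.
; Mouse X and Y axis events share one node that applies strongly scaled torque to the sphere, with the X component negated.
; The sphere's starting location is saved at BeginPlay as the respawn point.
; Pressing R calls Respawn, which moves the sphere back there and zeroes its linear and angular velocity.
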(event `self.ReceiveBeginPlay`
  (set `self.Respawn Location` (`SceneComponent.K2_GetComponentLocation` (`self.Sphere`))))

(event `Key|R`
  (params (Key :type "Key Structure" :default "AnyKey"))
  (:`Pressed`
    (`self.Respawn`)))

(event `InputAxisKey|MouseX`
  (params (AxisValue :type "Float (single-precision)"))
  (`PrimitiveComponent.AddTorque` (`self.Sphere`) (`KismetMathLibrary.MakeVector` (* (* AxisValue 1000000.0) -1.0) (* (stale `InputAxisKey|MouseY` AxisValue) 1000000.0)) "None" false :!label _label))

(event `InputAxisKey|MouseY`
  (params (AxisValue :type "Float (single-precision)"))
  (goto _label))

(fn `Respawn`
  (bind _sphere (`self.Sphere`))
  (`SceneComponent.K2_SetWorldLocation` _sphere (`self.Respawn Location`) false false)
  (`PrimitiveComponent.SetPhysicsAngularVelocity` _sphere (0.0 0.0 0.0) false "None")
  (`PrimitiveComponent.SetAllPhysicsLinearVelocity` _sphere (0.0 0.0 0.0) false))

(fn `UserConstructionScript`)